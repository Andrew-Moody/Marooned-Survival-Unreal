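; BP_MaroonedGameMode is the Marooned game mode that tracks connected players and provides player pawn spawning.
; It adds controllers to PlayerControllers on post-login and seamless-travel swaps, and removes them on logout.
; SpawnPlayer destroys any existing pawn, spawns a BP_GAS_PlayerCharacter at a random PlayerStart and possesses it.
; Nothing here calls SpawnPlayer, and an AI character spawn node is left unconnected.
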(event `self.ReceiveBeginPlay`)

(event `self.K2_PostLogin`
  (params (NewPlayer :type "PlayerController Object Reference"))
  ;[1 1 1] Store Players as they connect
  (`KismetArrayLibrary.Array_Add` (`self.PlayerControllers`) NewPlayer))

(event `self.K2_OnLogout`
  (params (ExitingController :type "Controller Object Reference"))
  ;[1 1 1] Remove Players as they disconnect
  (bind _asplayer_controller (cast `PlayerController` ExitingController))
  (`KismetArrayLibrary.Array_RemoveItem` (`self.PlayerControllers`) _asplayer_controller))

(event `self.K2_OnSwapPlayerControllers`
  (params (OldPC :type "PlayerController Object Reference") (NewPC :type "PlayerController Object Reference"))
  ;[1 1 1] Seamless Travel (Change Map)
  (`KismetArrayLibrary.Array_Add` (`self.PlayerControllers`) NewPC))

(fn `GetRandomPlayerStart`
  (returns (PlayerStartTransform :type "Transform Structure"))
  (bind _outactors (`GameplayStatics.GetAllActorsOfClass` "/Script/Engine.PlayerStart"))
  (return (`self.GetTransform` (`KismetArrayLibrary.Array_Random` _outactors))))

(fn `SpawnPlayer`
  (params (PlayerController :type "PlayerController Object Reference"))
  (locals (LocalPC :type "PlayerController Object Reference"))
  (bind _output_get (set `local.LocalPC` PlayerController))
  (bind _returnvalue (`Controller.K2_GetPawn` _output_get))
  ;[1 1 1] Destory Existing Pawn
  (`/Engine/EditorBlueprintResources/StandardMacros.IsValid` _returnvalue
    (:`Is Valid`
      (`self.K2_DestroyActor` _returnvalue))
    (:`Is Not Valid`
      _))
  (bind _returnvalue_2 (`|SpawnActorFromClass` "/Game/Marooned/Blueprints/GameplayAbilitySystem/BP_GAS_PlayerCharacter.BP_GAS_PlayerCharacter_C" (`self.GetRandomPlayerStart`) "Undefined" "OverrideRootScale" null null))
  (`Controller.Possess` (`local.LocalPC`) _returnvalue_2))

(fn `UserConstructionScript`)