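; Player controller for Marooned that handles spawning, HUD and inventory UI, item pickups and interaction prompts.
; The local controller requests a spawn from the game mode, creates widgets, then binds stats to the GAS player state after a one-second delay.
; The PawnPossessed RepNotify relays possession client-side, while authority-only overlaps add items to inventory or apply powerup GameplayEffects.
; A per-tick forward trace updates the HUD's interact text from BPI_Interactable targets.
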(event `self.ReceiveTick`
  (params (DeltaSeconds :type "Float (single-precision)"))
  (if (`self.IsLocalPlayerController`)
    (`self.UpdateLookTarget`)))

(event `Event CreateHUD`
  ;[1 1 1] Ideally this should be moved to HUD
  (`|ExecutionSequence`
    (:`then_0`
      (bind _asbp_hud (cast `/Game/Marooned/Blueprints/Core/BP_HUD` (`self.GetHUD`))
        (:`then`
          (set `self.BP_HUD` _asbp_hud))
        (:`CastFailed`
          (`KismetSystemLibrary.PrintString` "Failed to find HUD"))))
    (:`then_1`
      (bind _returnvalue (`|CreateWidget` "/Game/Marooned/Blueprints/UI/WB_Info.WB_Info_C" self))
      (bind _output_get (set `self.WB_Info` _returnvalue))
      (`UserWidget.AddToViewport` _output_get 0))
    (:`then_3`
      (bind _returnvalue_2 (`|CreateWidget` "/Game/Marooned/Blueprints/Inventory/WB_Inventory.WB_Inventory_C" self))
      (bind _output_get_2 (set `self.WB_Inventory` _returnvalue_2))
      (`UserWidget.AddToViewport` _output_get_2 0)
      (`/Game/Marooned/Blueprints/Inventory/WB_Inventory.Event SetTarget` _output_get_2 (`self.BP_Inventory`))
      (`/Game/Marooned/Blueprints/Inventory/WB_CraftingMenu.Event SetTarget` (`/Game/Marooned/Blueprints/Inventory/WB_Inventory.WB_CraftingMenu` (`self.WB_Inventory`)) (`self.BP_Inventory`) (`|MakeArray` (make `/Game/Marooned/Blueprints/Inventory/F_Recipe` (make `/Game/Marooned/Blueprints/Item/F_ItemSlot` "BP_DA_Item_C:DA_Item_BloodwoodLog" 1) (`|MakeArray` (make `/Game/Marooned/Blueprints/Item/F_ItemSlot` "BP_DA_Item_C:DA_Item_SpruceLog" 1) :!type "/Game/Marooned/Blueprints/Item/F_ItemSlot Structure")) (make `/Game/Marooned/Blueprints/Inventory/F_Recipe` (make `/Game/Marooned/Blueprints/Item/F_ItemSlot` "BP_DA_Item_C:DA_Item_SpruceLog" 1) (`|MakeArray` (make `/Game/Marooned/Blueprints/Item/F_ItemSlot` "BP_DA_Item_C:DA_Item_BloodwoodLog" 1) :!type "/Game/Marooned/Blueprints/Item/F_ItemSlot Structure")) :!type "/Game/Marooned/Blueprints/Inventory/F_Recipe Structure")))
    (:`then_4`
      (bind _returnvalue_3 (`|GenericCreateObject` "/Game/Marooned/Blueprints/UI/WB_StatsTest.WB_StatsTest_C"))
      (bind _output_get_3 (set `self.WB_StatsTest` _returnvalue_3))
      (`UserWidget.AddToViewport` _output_get_3 0))))

(event `self.ReceiveBeginPlay`
  (`KismetSystemLibrary.PrintText` (`|FormatText` "Begin PC, IsLocal: {Local}, HasAuth: {Auth}" (`self.IsLocalPlayerController`) (`self.HasAuthority`)) true true (struct :`G` 0.66 :`B` 1.0 :`A` 1.0) 30.0)
  (if (`self.IsLocalPlayerController`)
    (`self.SR_SpawnPlayer`)
    (`self.Event CreateHUD`)
    ;[1 1 1] Seems there isn't an easy way to ensure order that BeginPlay is called. This delay should ensure everything has done any self initialization
    (`KismetSystemLibrary.Delay` 1.0)
    (`self.Event SetupPlayer`)))

(event `SR_SpawnPlayer`
  (bind _asbp_marooned_game_mode (cast `/Game/Marooned/Blueprints/Core/BP_MaroonedGameMode` (`GameplayStatics.GetGameMode`)))
  (`/Game/Marooned/Blueprints/Core/BP_MaroonedGameMode.SpawnPlayer` _asbp_marooned_game_mode self))

(event `Key|P`
  (params (Key :type "Key Structure"))
  (:`Pressed`
    (`self.SR_SpawnPlayer`)))

(event `Event ClientOnPossess`
  (params (`Possesed Pawn` :type "Pawn Object Reference"))
  (`KismetSystemLibrary.PrintText` (`|FormatText` "Pawn Possessed, Valid PlayerState: {Valid}" (`KismetSystemLibrary.IsValid` (`Pawn.PlayerState` `Possesed Pawn`))) true true (struct :`G` 0.66 :`B` 1.0 :`A` 1.0) 30.0)
  (bind _asbp_gas_player_character (cast `/Game/Marooned/Blueprints/GameplayAbilitySystem/BP_GAS_PlayerCharacter` `Possesed Pawn`))
  (set `self.BP_GAS_PlayerCharacter` _asbp_gas_player_character))

(event `Event SetupPlayer`
  (`KismetSystemLibrary.PrintText` (`|FormatText` "Setup Player IsLocal: {Local}, HasAuth: {Auth}" (`self.IsLocalPlayerController`) (`self.HasAuthority`)) true true (struct :`G` 0.66 :`B` 1.0 :`A` 1.0) 30.0)
  (bind _bp_gas_playercharacter (`self.BP_GAS_PlayerCharacter`)
    (:`then`
      (bind _asbp_gas_player_state (cast `/Game/Marooned/Blueprints/GameplayAbilitySystem/BP_GAS_PlayerState` (`Pawn.PlayerState` _bp_gas_playercharacter)))
      (bind _output_get (set `self.As BP GAS Player State` _asbp_gas_player_state))
      (`/Game/Marooned/Blueprints/UI/WB_StatsPanel.Event SetTarget` (`/Game/Marooned/Blueprints/UI/WB_StatsTest.WB_StatsPanel` (`self.WB_StatsTest`)) _output_get)
      (set `/Game/Marooned/Blueprints/GameplayAbilitySystem/BP_GAS_PlayerCharacter.WB_WorldCanvas` (`/Game/Marooned/Blueprints/Core/BP_HUD.WB_WorldCanvas` (`self.BP_HUD`)) _bp_gas_playercharacter))
    (:`else`)))

(event `Event ClientUnPossess`
  (params (UnpossessedPawn :type "Pawn Object Reference")))

(event `self.ReceivePossess`
  (params (PossessedPawn :type "Pawn Object Reference"))
  (add `self.OnActorBeginOverlap` PossessedPawn (delegate `Event CharacterBeginOverlap`))
  (set `self.bPawnPossessed` true))

(event `self.ReceiveUnPossess`
  (params (UnpossessedPawn :type "Pawn Object Reference"))
  (remove `self.OnActorBeginOverlap` UnpossessedPawn (delegate `Event CharacterBeginOverlap`))
  (set `self.bPawnPossessed` false))

(event `Event CharacterBeginOverlap` :!signature `self.OnActorBeginOverlap`
  (params (OverlappedActor :type "Actor Object Reference") (OtherActor :type "Actor Object Reference"))
  (`/Engine/EditorBlueprintResources/ActorMacros.Switch Has Authority`
    (:`Authority`
      (bind _asbp_world_item (cast `/Game/Marooned/Blueprints/Item/BP_WorldItem` OtherActor)
        (:`then`
          (`self.Event CollectItem` _asbp_world_item))
        (:`CastFailed`
          (bind _asbp_powerup (cast `/Game/Marooned/Blueprints/Powerups/BP_Powerup` OtherActor))
          (`self.Event CollectPowerup` _asbp_powerup))))))

(event `Event CollectItem`
  (params (WorldItem :type "/Game/Marooned/Blueprints/Item/BP_WorldItem Object Reference"))
  (`/Engine/EditorBlueprintResources/ActorMacros.Switch Has Authority`
    (:`Authority`
      (`/Game/Marooned/Blueprints/Core/BP_Inventory.Server AddItem` (`self.BP_Inventory`) (`/Game/Marooned/Blueprints/Item/BP_WorldItem.GetItem` WorldItem) (`/Game/Marooned/Blueprints/Item/BP_WorldItem.GetAssetId` WorldItem) 1)
      (`self.K2_DestroyActor` WorldItem))))

(event `Event CollectPowerup`
  (params (Powerup :type "/Game/Marooned/Blueprints/Powerups/BP_Powerup Object Reference"))
  (`/Engine/EditorBlueprintResources/ActorMacros.Switch Has Authority`
    (:`Authority`
      (bind _asbp_gas_player_character (cast `/Game/Marooned/Blueprints/GameplayAbilitySystem/BP_GAS_PlayerCharacter` (`self.K2_GetPawn`)))
      (bind _returnvalue (`AbilitySystemBlueprintLibrary.GetAbilitySystemComponent` _asbp_gas_player_character))
      (bind _asmarooned_ability_system_component (cast `MaroonedAbilitySystemComponent` _returnvalue))
      (`AbilitySystemComponent.BP_ApplyGameplayEffectToSelf` _asmarooned_ability_system_component (`/Game/Marooned/Blueprints/Powerups/BP_Powerup.Effect` Powerup) 0.0 (`AbilitySystemComponent.MakeEffectContext` _returnvalue))
      (`self.K2_DestroyActor` Powerup))))

(event `InputAction|Inventory` :paused true
  (params (Key :type "Key Structure"))
  (:`Pressed`
    (`self.Event ToggleInventory`)))

(event `Event ChangeItemCount`
  (params (ItemCount :type Integer))
  (`KismetSystemLibrary.PrintText` (`|FormatText` "PlayerController Change Count: {Count}" ItemCount))
  (`/Game/Marooned/Blueprints/UI/WB_ItemCount.Event ChangeCount` (`self.WB_ItemCount`) 0 ItemCount))

(event `Event ToggleInventory`
  (`/Engine/EditorBlueprintResources/StandardMacros.FlipFlop`
    (:`A`
      (`self.EnableInput` (`self.K2_GetPawn`) self)
      (`WidgetBlueprintLibrary.SetInputMode_GameOnly` self)
      (set `self.bShowMouseCursor` false)
      (`Widget.SetVisibility` (`self.WB_Inventory`) "Collapsed"))
    (:`B`
      (`self.DisableInput` (`self.K2_GetPawn` self) self)
      (`WidgetBlueprintLibrary.SetInputMode_GameAndUIEx` self (`self.WB_Inventory`))
      (set `self.bShowMouseCursor` true)
      (`Widget.SetVisibility` (`self.WB_Inventory`) "Visible"))))

(fn `OnRep_bPawnPossessed`
  (bind _returnvalue (`GameplayStatics.GetPlayerPawn` 0))
  (if (`self.IsLocalPlayerController`)
    (if (`self.bPawnPossessed`)
      (`self.Event ClientOnPossess` _returnvalue)
      (else
        (`self.Event ClientUnPossess` _returnvalue)))))

(fn `UpdateLookTarget`
  (bind _returnvalue (`GameplayStatics.GetPlayerCharacter` 0))
  (bind _returnvalue_2 (`self.K2_GetActorLocation` _returnvalue))
  (`/Engine/EditorBlueprintResources/StandardMacros.IsValid` _returnvalue
    (:`Is Valid`
      (bind (_outhit _returnvalue_3) (`KismetSystemLibrary.LineTraceSingle` _returnvalue_2 (+ _returnvalue_2 (* (`self.GetActorForwardVector` _returnvalue) 300.0)) "TraceTypeQuery1"))
      (bind (_bblockinghit _binitialoverlap _time _distance _location _impactpoint _normal _impactnormal _physmat _hitactor) (`GameplayStatics.BreakHitResult` _outhit))
      (if (!= _hitactor (`self.LookTarget`))
        (bind _output_get (set `self.LookTarget` _hitactor))
        (bind _asbpi_interactable (cast `/Game/Marooned/Blueprints/Interaction/BPI_Interactable` _output_get)
          (:`then`
            (bind _text (`/Game/Marooned/Blueprints/Interaction/BPI_Interactable.GetText` _asbpi_interactable))
            (`/Game/Marooned/Blueprints/Core/BP_HUD.Event SetInteractInfo` (`self.BP_HUD`) _text))
          (:`CastFailed`
            (`/Game/Marooned/Blueprints/Core/BP_HUD.Event SetInteractInfo` (`self.BP_HUD`) "")))))))

(fn `UserConstructionScript`)