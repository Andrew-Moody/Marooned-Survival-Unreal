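; Enemy character Blueprint for Marooned, with a sword-slash style attack and a basic health pool.
; Attack writes the slash montage and current time into a replicated montage struct, whose OnRep plays it with the struct's play rate and start section.
; A second Attack event takes damage and subtracts it from clamped Health.
; The zero-health branch is empty, so no death handling exists yet.
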(event `self.ReceiveBeginPlay`)

(event `Event Attack`
  (bind _structout (setmembers `/Game/Marooned/Blueprints/Core/F_MontageData` :`StructRef` (`self.AttackMontage`) :`Montage` "/Game/Marooned/Characters/Man/AM_Man_Slash.AM_Man_Slash" :`StartTime` (`GameplayStatics.GetTimeSeconds`)))
  (set `self.AttackMontage` _structout))

(event `/Game/Marooned/Blueprints/WorldGen/BPI_Attack.Attack`
  (params (HitResult :type "HitResult Structure") (Damage :type "Float (double-precision)"))
  (bind _output_get (set `self.Health` (`KismetMathLibrary.FClamp` (- (`self.Health`) Damage) 0.0 10.0)))
  (if (<= _output_get 0.0)
    _))

(fn `OnRep_AttackMontage`
  (bind (_montage _starttime _playrate _startsection) (break `/Game/Marooned/Blueprints/Core/F_MontageData` (`self.AttackMontage`)))
  (`self.PlayAnimMontage` _montage _playrate _startsection))

(fn `UserConstructionScript`)