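; Slot-based multiplayer inventory that stores item stacks and handles adding, swapping and single-ingredient crafting.
; Server events apply adds and swaps, then Client events replay them on remote machines, and refresh calls report changed slots.
; Adding stacks onto a matching item or fills the first empty slot.
; Crafting checks only the recipe's first input, and lookups use FindItem and FindEmpty macros built on a two-gate Latch.
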(event `self.ReceiveBeginPlay`
  (for _ (range (`self.Size`))
    (`KismetArrayLibrary.Array_Add` (`self.Items`) (make `/Game/Marooned/Blueprints/Item/F_ItemSlot` (struct)))))

(event `Event RefreshAll`
  (for _index (range (`self.Size`))
    (`self.OnInventoryRefresh` _index (`|GetArrayItem` (`self.Items`) _index))))

(event `Server AddItem`
  (params (AssetId :type "PrimaryAssetId Structure") (Count :type Integer))
  (`self.AddItem` AssetId Count)
  (`self.Client AddItem` AssetId Count))

(event `Client AddItem`
  (params (AssetId :type "PrimaryAssetId Structure") (Count :type Integer))
  (`/Engine/EditorBlueprintResources/ActorComponentMacros.Switch Has Authority`
    (:`Remote`
      (`self.AddItem` AssetId Count))))

(event `Client UpdateSlot`
  (params (Index :type Integer) (Item :type "/Game/Marooned/Blueprints/Item/F_ItemSlot Structure"))
  (`KismetArrayLibrary.Array_Set` (`self.Items`) Index Item)
  (`self.OnInventoryRefresh` Index Item))

(event `Server SwapSlots`
  (params (SlotA :type Integer) (SlotB :type Integer))
  (`self.SwapSlots` SlotA SlotB)
  (`self.Client SwapSlots` SlotA SlotB))

(event `Client SwapSlots`
  (params (SlotA :type Integer) (SlotB :type Integer))
  (`/Engine/EditorBlueprintResources/ActorComponentMacros.Switch Has Authority`
    (:`Remote`
      (`self.SwapSlots` SlotA SlotB))))

(event `Server CraftItem`
  (params (Recipe :type "/Game/Marooned/Blueprints/Inventory/F_Recipe Structure"))
  (bind (_outputitem _inputitems) (break `/Game/Marooned/Blueprints/Inventory/F_Recipe` Recipe))
  (bind (_itemid _count) (break `/Game/Marooned/Blueprints/Item/F_ItemSlot` _outputitem))
  (bind (_itemid_2 _count_2) (break `/Game/Marooned/Blueprints/Item/F_ItemSlot` (`|GetArrayItem` _inputitems)))
  (`KismetSystemLibrary.PrintString` "Crafting")
  (bind _index (`self.FindItem` _itemid_2)
    (:`Found`
      (`KismetSystemLibrary.PrintText` (`|FormatText` "Found Item at {Index}" _index))
      (bind _output (`|GetArrayItem` (`self.Items`) _index))
      (bind (_itemid_3 _count_3) (break `/Game/Marooned/Blueprints/Item/F_ItemSlot` _output))
      (if (<= _count_2 _count_3)
        (`KismetSystemLibrary.PrintString` "Sufficient Quantity")
        (bind _returnvalue (- _count_3 _count_2))
        (bind _structout (setmembers `/Game/Marooned/Blueprints/Item/F_ItemSlot` :`StructRef` _output :`ItemId` (select `bool` (> _returnvalue 0) :`true` _itemid_3) :`Count` _returnvalue))
        (`self.Client UpdateSlot` _index _structout)
        (`self.Server AddItem` _itemid _count)
        (else
          (`KismetSystemLibrary.PrintString` "InSufficient Quantity"))))
    (:`NotFound`
      (`KismetSystemLibrary.PrintText` (`|FormatText` "Missing Required Item {Item}" (`KismetSystemLibrary.Conv_PrimaryAssetIdToString` _itemid_2))))))

(fn `AddItem`
  (params (ItemId :type "PrimaryAssetId Structure") (Count :type Integer))
  (returns (bSuccess :type Boolean))
  (locals (LocalItem :type "/Game/Marooned/Blueprints/Item/F_ItemSlot Structure"))
  (bind _f_itemslot (make `/Game/Marooned/Blueprints/Item/F_ItemSlot` ItemId Count))
  (`KismetSystemLibrary.PrintText` (`|FormatText` "Adding {Count} {Name}" Count (`KismetSystemLibrary.Conv_PrimaryAssetIdToString` ItemId)))
  (bind _index (`self.FindItem` ItemId)
    (:`Found`
      (`KismetSystemLibrary.PrintString` "Found Item")
      (bind _output (`|GetArrayItem` (`self.Items`) _index))
      (bind _structout (setmembers `/Game/Marooned/Blueprints/Item/F_ItemSlot` :`StructRef` _output :`Count` (+ (`.Count_4_69ABB6D944FDFFC50CD5FAB9746F251E` (break `/Game/Marooned/Blueprints/Item/F_ItemSlot` _output)) Count)))
      (`self.OnInventoryRefresh` _index _structout))
    (:`NotFound`
      (bind _index_2 (`self.FindEmpty`)
        (:`Found`
          (`KismetSystemLibrary.PrintString` "Found Empty")
          (`KismetArrayLibrary.Array_Set` (`self.Items`) _index_2 _f_itemslot)
          (`self.OnInventoryRefresh` _index_2 _f_itemslot))
        (:`NotFound`
          (`KismetSystemLibrary.PrintString` "Inv Full")
          (return false)))))
  (return true))

(fn `OnRep_CountCheck`
  (`KismetSystemLibrary.PrintString` "OnRep CountCheck"))

(fn `OnRep_Items`
  (`KismetSystemLibrary.PrintString` "RepNotify Items"))

(fn `SwapSlots`
  (params (SlotA :type Integer) (SlotB :type Integer))
  (locals (TempItem :type "/Game/Marooned/Blueprints/Item/F_ItemSlot Structure"))
  (bind _items (`self.Items`))
  (bind _slota (`local.SlotA`))
  (bind _slotb (`local.SlotB`))
  (set `local.TempItem` (`|GetArrayItem` (`self.Items`) SlotA))
  (`KismetArrayLibrary.Array_Set` _items (`local.SlotA`) (`|GetArrayItem` _items (`local.SlotB`)))
  (`KismetArrayLibrary.Array_Set` (`self.Items`) (`local.SlotB`) (`local.TempItem`))
  (`self.OnInventoryRefresh` _slota (`|GetArrayItem` (`self.Items`) _slota))
  (`self.OnInventoryRefresh` _slotb (`|GetArrayItem` (`self.Items`) _slotb)))