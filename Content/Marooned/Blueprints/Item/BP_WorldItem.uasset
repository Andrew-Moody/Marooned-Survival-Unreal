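; BP_WorldItem is an item placed in the world whose appearance comes from an item data asset.
; The DataAsset RepNotify applies the asset's mesh to the StaticMesh component when valid and prints the mesh name.
; GetAssetId exposes the data asset's Primary Asset ID to callers.
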(fn `GetAssetId`
  (returns (AssetId :type "PrimaryAssetId Structure"))
  (return (`KismetSystemLibrary.GetPrimaryAssetIdFromObject` (`self.DataAsset`))))

(fn `OnRep_DataAsset`
  (bind _mesh (`/Game/Marooned/Blueprints/Item/BP_DA_Item.Mesh` (`self.DataAsset`)))
  (`/Engine/EditorBlueprintResources/StandardMacros.IsValid` (`self.DataAsset`)
    (:`Is Valid`
      (`StaticMeshComponent.SetStaticMesh` (`self.StaticMesh`) _mesh)
      (`KismetSystemLibrary.PrintString` (`KismetSystemLibrary.GetObjectName` _mesh)))))

(fn `UserConstructionScript`)