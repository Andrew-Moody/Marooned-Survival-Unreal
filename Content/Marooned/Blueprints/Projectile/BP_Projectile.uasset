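; Gameplay Ability System projectile that damages or debuffs actors it overlaps, with knockback.
; Launch sets movement velocity on the authority.
; Authority-side sphere overlap skips the Instigator, applies the supplied effect spec with a constructed hit result to targets with an ability system component, and sends a knockback gameplay event.
; It then spawns Niagara death effects through ClientsPlayDeathEffects and destroys itself.
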(event `self.ReceiveBeginPlay`)

(event `Event Launch`
  (params (Direction :type "Vector Structure"))
  (bind _projectilemovement (`self.ProjectileMovement`))
  (`/Engine/EditorBlueprintResources/ActorMacros.Switch Has Authority`
    (:`Authority`
      (set `MovementComponent.Velocity` (* Direction (`ProjectileMovementComponent.InitialSpeed` _projectilemovement)) _projectilemovement))))

(event `self.Sphere.OnComponentBeginOverlap`
  (params (OverlappedComponent :type "PrimitiveComponent Object Reference") (OtherActor :type "Actor Object Reference") (OtherComp :type "PrimitiveComponent Object Reference") (OtherBodyIndex :type Integer) (bFromSweep :type Boolean) (SweepResult :type "HitResult Structure (by ref)"))
  (bind _returnvalue (`AbilitySystemBlueprintLibrary.GetAbilitySystemComponent` OtherActor))
  (bind _returnvalue_2 (`ActorComponent.GetOwner` _returnvalue))
  (`/Engine/EditorBlueprintResources/ActorMacros.Switch Has Authority`
    (:`Authority`
      (if (not (== OtherActor (`self.Instigator`)))
        (`/Engine/EditorBlueprintResources/StandardMacros.IsValid` _returnvalue
          (:`Is Valid`
            (if true
              (bind _returnvalue_3 (`AbilitySystemBlueprintLibrary.GetEffectContext` (`self.EffectSpecHandle`)))
              (`AbilitySystemBlueprintLibrary.EffectContextAddHitResult` _returnvalue_3 (`GameplayStatics.MakeHitResult` false false 0.0 0.0 (0.0 0.0 0.0) (0.0 0.0 0.0) (0.0 0.0 1.0) (0.0 0.0 1.0) null OtherActor OtherComp "None" "None" OtherBodyIndex))
              (`AbilitySystemComponent.BP_ApplyGameplayEffectSpecToSelf` _returnvalue (`self.EffectSpecHandle`))
              (`AbilitySystemBlueprintLibrary.SendGameplayEventToActor` _returnvalue_2 (struct :`TagName` "Event.Debuff.Knockback") (make `GameplayEventData` (struct :`TagName` "Event.Debuff.Knockback") (`self.Instigator`) _returnvalue_2))
              (`self.Clients PlayDeathEffects`)
              (`self.K2_DestroyActor`)
              (else
                (`KismetSystemLibrary.PrintString` "Not from sweep")))))))))

(event `Clients PlayDeathEffects`
  (bind (_returnvalue_location _returnvalue_rotation _returnvalue_scale) (`KismetMathLibrary.BreakTransform` (`self.GetTransform`)))
  (`NiagaraFunctionLibrary.SpawnSystemAtLocation` (`self.NiagaraSystem`) _returnvalue_location _returnvalue_rotation _returnvalue_scale))

(fn `UserConstructionScript`)