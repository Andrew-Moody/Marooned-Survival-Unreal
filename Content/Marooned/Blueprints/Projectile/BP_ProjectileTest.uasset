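; BP_ProjectileTest is a test projectile that moves manually and prints what it hits.
; Launch sets velocity from direction and speed, then Tick integrates position and applies acceleration.
; Each tick sphere-traces from old to new position with debug drawing, since movement is unswept; actor overlaps also print.
; BeginPlay tints the sphere through a dynamic material, using different colors for authority and remote copies.
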(event `self.ReceiveBeginPlay`
  (`self.SetActorTickEnabled` true)
  (`/Engine/EditorBlueprintResources/ActorMacros.Switch Has Authority`
    (:`Authority`
      (`self.Event SetColor` (struct :`R` 1.0 :`B` 0.007179 :`A` 0.571)))
    (:`Remote`
      (`self.Event SetColor` (struct :`G` 1.0 :`B` 0.154823 :`A` 0.596)))))

(event `Event Launch`
  (params (Direction :type "Vector Structure"))
  (set `self.Velocity` (* Direction (`self.Speed`)))
  (`self.SetActorTickEnabled` true))

(event `Event SetColor`
  (params (Color :type "LinearColor Structure"))
  (bind _returnvalue (`PrimitiveComponent.CreateDynamicMaterialInstance` (`self.Sphere`) 0 "/Game/Marooned/Characters/M_SolidColor.M_SolidColor" "None"))
  (`MaterialInstanceDynamic.SetVectorParameterValue` _returnvalue "BaseColor" Color))

(event `self.ReceiveActorBeginOverlap`
  (params (OtherActor :type "Actor Object Reference"))
  (`KismetSystemLibrary.PrintText` (`|FormatText` "Hit {Actor}" (`KismetSystemLibrary.GetObjectName` OtherActor))))

(event `self.ReceiveTick`
  (params (DeltaSeconds :type "Float (single-precision)"))
  (set `self.CurrentPos` (`self.K2_GetActorLocation`))
  (bind _output_get (set `self.NewPos` (+ (* DeltaSeconds (`self.Velocity`)) (`self.CurrentPos`))))
  (`self.K2_SetActorLocation` _output_get)
  (`self.Event UpdateVelocity` DeltaSeconds)
  (bind (_outhit _returnvalue) (`KismetSystemLibrary.SphereTraceSingleByProfile` :`Start` (`self.CurrentPos`) :`End` (`self.NewPos`) :`Radius` (`self.Radius`) :`ProfileName` "BlockAllDynamic" :`DrawDebugType` "ForDuration"))
  (if _returnvalue
    (`KismetSystemLibrary.PrintText` (`|FormatText` "Hit {Name}" (`KismetSystemLibrary.GetObjectName` (`.HitActor` (`GameplayStatics.BreakHitResult` _outhit)))))))

(event `Event UpdateVelocity`
  (params (DeltaSeconds :type "Float (double-precision)"))
  (set `self.Velocity` (+ (`self.Velocity`) (* (`self.Acceleration`) DeltaSeconds))))

(fn `UserConstructionScript`)