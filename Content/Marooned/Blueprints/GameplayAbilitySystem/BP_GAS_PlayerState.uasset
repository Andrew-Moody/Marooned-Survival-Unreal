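; Player state for Marooned that owns the player's Gameplay Ability System setup and relays health changes.
; On the server at BeginPlay it applies an initial stats effect and grants knockback, death and melee attack abilities.
; Health changes notify listeners, refresh the pawn's health display and send a death event at zero.
; It also toggles a test equipment effect and routes primary input to an override ability, falling back to melee.
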(event `self.ReceiveBeginPlay`
  (`/Engine/EditorBlueprintResources/ActorMacros.Switch Has Authority`
    (:`Authority`
      (set `self.ASC` (`AbilitySystemBlueprintLibrary.GetAbilitySystemComponent` self))
      (`AbilitySystemComponent.BP_ApplyGameplayEffectToSelf` (`self.ASC`) "/Game/Marooned/Blueprints/GameplayAbilitySystem/Effects/BP_GE_InitializeStats.BP_GE_InitializeStats_C" 0.0 (make `GameplayEffectContextHandle`))
      (`AbilitySystemComponent.K2_GiveAbility` (`self.ASC`) "/Game/Marooned/Blueprints/GameplayAbilitySystem/Abilities/BP_GA_Knockback.BP_GA_Knockback_C" 0 -1)
      (`AbilitySystemComponent.K2_GiveAbility` (`self.ASC`) "/Game/Marooned/Blueprints/GameplayAbilitySystem/Abilities/BP_GA_Death.BP_GA_Death_C" 0 -1)
      (`AbilitySystemComponent.K2_GiveAbility` (`self.ASC`) "/Game/Marooned/Blueprints/GameplayAbilitySystem/Abilities/BP_GA_MeleeAttack.BP_GA_MeleeAttack_C" 0 1))))

(event `self.RecieveHealthChanged`
  (params (NewValue :type "Float (single-precision)") (OldValue :type "Float (single-precision)"))
  (`self.HealthUpdated` NewValue OldValue)
  (`self.Clients UpdateHealth`)
  (if (and (<= NewValue 0.0) (`KismetSystemLibrary.IsServer`))
    (`AbilitySystemBlueprintLibrary.SendGameplayEventToActor` self (struct :`TagName` "Event.Death"))))

(event `Event EquipItem`
  (`self.Event UnequipItem`)
  (bind _returnvalue (`AbilitySystemComponent.BP_ApplyGameplayEffectToSelf` (`self.ASC`) "/Game/Marooned/Blueprints/GameplayAbilitySystem/Effects/BP_GE_EquipItemTest.BP_GE_EquipItemTest_C" 0.0 (make `GameplayEffectContextHandle`)))
  (set `self.EquipmentEffect` _returnvalue)
  (set `self.bItemEquipped` true))

(event `self.RecieveMaxHealthChanged`
  (params (NewValue :type "Float (single-precision)") (OldValue :type "Float (single-precision)"))
  (`self.MaxHealthUpdated` NewValue OldValue)
  (`self.Clients UpdateHealth`))

(event `Clients UpdateHealth`
  (bind _asbp_gas_player_character (cast `/Game/Marooned/Blueprints/GameplayAbilitySystem/BP_GAS_PlayerCharacter` (`self.GetPawn`)))
  (`/Game/Marooned/Blueprints/GameplayAbilitySystem/BP_GAS_PlayerCharacter.Event RefreshHealth` _asbp_gas_player_character))

(event `Event UnequipItem`
  (if (`self.bItemEquipped`)
    (`AbilitySystemComponent.RemoveActiveGameplayEffect` (`self.ASC`) (`self.EquipmentEffect`) -1)
    (set `self.bItemEquipped` false)))

(event `Event ActivatePrimaryAbility`
  (bind _asc (`self.ASC`))
  (bind _outabilityhandles (`AbilitySystemComponent.FindAllAbilitiesWithInputID` _asc 2))
  (if (> (`KismetArrayLibrary.Array_Length` _outabilityhandles) 0)
    (`AbilitySystemComponent.PressInputID` _asc 2)
    (else
      (`AbilitySystemComponent.PressInputID` _asc 1))))

(fn `UserConstructionScript`)