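; Base AI character for the Gameplay Ability System that handles ability granting, attacking, health and death.
; On BeginPlay it applies a stat initializer effect, then grants knockback, death and its configured abilities, the latter all on one input ID that Attack presses.
; Health and tag changes are relayed through dispatchers, tags only on authority, and zero health sends a death gameplay event.
; A Ragdoll event switches the mesh to physics and disables capsule collision.
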(event `self.ReceiveBeginPlay`
  (set `self.ASC` (`AbilitySystemBlueprintLibrary.GetAbilitySystemComponent` self))
  (`AbilitySystemComponent.BP_ApplyGameplayEffectToSelf` (`self.ASC`) (`self.StatInitializer`) 0.0 (make `GameplayEffectContextHandle`))
  (`AbilitySystemComponent.K2_GiveAbility` (`self.ASC`) "/Game/Marooned/Blueprints/GameplayAbilitySystem/Abilities/BP_GA_Knockback.BP_GA_Knockback_C" 0 -1)
  (`AbilitySystemComponent.K2_GiveAbility` (`self.ASC`) "/Game/Marooned/Blueprints/GameplayAbilitySystem/Abilities/BP_GA_Death.BP_GA_Death_C" 0 -1)
  (for (_array_element _array_index) (`self.Abilities`)
    (`AbilitySystemComponent.K2_GiveAbility` (`self.ASC`) _array_element (+ _array_index 1) 1)
    (`KismetSystemLibrary.PrintText` (`|FormatText` "Added Ability: {Ability}" (`KismetSystemLibrary.GetClassDisplayName` _array_element)))))

(event `Event Attack`
  (`AbilitySystemComponent.PressInputID` (`self.ASC`) 1))

(event `self.RecieveHealthChanged`
  (params (NewHealth :type "Float (single-precision)") (OldHealth :type "Float (single-precision)"))
  (`|ExecutionSequence`
    (:`then_0`
      (`self.HealthChanged` NewHealth (`.ReturnValue` (`AbilitySystemBlueprintLibrary.GetFloatAttributeFromAbilitySystemComponent` (`self.ASC`) (struct :`AttributeName` "MaxHealth" :`Attribute` "/Script/Marooned.MaroonedAttributeSet:MaxHealth" :`AttributeOwner` "/Script/CoreUObject.Class'\"/Script/Marooned.MaroonedAttributeSet\"'"))))
      (if (<= NewHealth 0.0)
        (`AbilitySystemBlueprintLibrary.SendGameplayEventToActor` self (struct :`TagName` "Event.Death"))
        (`self.DeathEventDispatcher`)))))

(event `Event Ragdoll`
  (`PrimitiveComponent.SetSimulatePhysics` (`self.Mesh`) true)
  ;[1 1 1] To Stop Animation
  (`ActorComponent.SetComponentTickEnabled` (`self.Mesh`) false)
  (`PrimitiveComponent.SetCollisionEnabled` (`self.CapsuleComponent`) "NoCollision"))

(event `self.RecieveTagChanged`
  (params (ChangedTag :type "GameplayTag Structure") (NewCount :type Integer))
  (`/Engine/EditorBlueprintResources/ActorMacros.Switch Has Authority`
    (:`Authority`
      (`self.TagChanged` ChangedTag NewCount))))

(fn `UserConstructionScript`)