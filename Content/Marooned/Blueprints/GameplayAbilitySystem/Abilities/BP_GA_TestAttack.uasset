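; Test melee attack gameplay ability that plays a slash montage, waits for a melee attack gameplay event, then targets actors near the avatar.
; An instant radius target actor, filtered to exclude self, gathers nearby actors.
; Each one with an ability system component receives a test gameplay effect and a knockback debuff event.
; Debug prints trace each step, and the ability ends when the montage finishes, blends out or is cancelled.
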(event `self.K2_ActivateAbility`
  (bind _returnvalue (`self.GetAvatarActorFromActorInfo`))
  (`KismetSystemLibrary.PrintText` (`|FormatText` "Activate TestAttack") true true (struct :`R` 1.0 :`A` 1.0) 5.0)
  (`AbilityTask_PlayMontageAndWait.CreatePlayMontageAndWaitProxy` "None" "/Game/Marooned/Characters/Man/AM_Man_Slash.AM_Man_Slash"
    (:`then`
      (`AbilityTask_WaitGameplayEvent.WaitGameplayEvent` (struct :`TagName` "Event.Attack.Melee") null
        (:`EventReceived`
          (bind (_asynctaskproxy _data) (`AbilityTask_WaitTargetData.WaitTargetData` "None" "Instant" "/Script/GameplayAbilities.GameplayAbilityTargetActor_Radius" 100.0 (make `GameplayAbilityTargetingLocationInfo` "ActorTransform" "0.000000,0.000000,0.000000|0.000000,0.000000,-0.000000|1.000000,1.000000,1.000000" _returnvalue) (struct) null (`AbilitySystemBlueprintLibrary.MakeFilterHandle` (make `GameplayTargetDataFilter` null "TDFS_NoSelf") _returnvalue))
            (:`ValidData`
              (`KismetSystemLibrary.PrintString` "Valid Data" true true (struct :`R` 1.0 :`A` 1.0) 5.0)
              (for _array_element (`AbilitySystemBlueprintLibrary.GetAllActorsFromTargetData` _data)
                (bind _returnvalue_2 (`AbilitySystemBlueprintLibrary.GetAbilitySystemComponent` _array_element))
                (`/Engine/EditorBlueprintResources/StandardMacros.IsValid` _returnvalue_2
                  (:`Is Valid`
                    (`KismetSystemLibrary.PrintText` (`|FormatText` "Targeting detected {Actor} with ASC" _array_element) true true (struct :`R` 1.0 :`A` 1.0) 5.0)
                    (`AbilitySystemComponent.BP_ApplyGameplayEffectToSelf` _returnvalue_2 "/Game/Marooned/Blueprints/GameplayAbilitySystem/Effects/BP_GE_TestEffect.BP_GE_TestEffect_C" 0.0 (make `GameplayEffectContextHandle`))
                    (bind _returnvalue_3 (`ActorComponent.GetOwner` _returnvalue_2))
                    (`AbilitySystemBlueprintLibrary.SendGameplayEventToActor` _returnvalue_3 (struct :`TagName` "Event.Debuff.Knockback") (make `GameplayEventData` (struct :`TagName` "Event.Debuff.Knockback") (`self.GetAvatarActorFromActorInfo`) _array_element))
                    (`KismetSystemLibrary.PrintText` (`|FormatText` "Sent Event to {Actor} (with authority: {Authority})" _returnvalue_3 (`Actor.HasAuthority` _returnvalue_3)) true true (struct :`G` 1.0 :`A` 1.0) 5.0))
                  (:`Is Not Valid`
                    (`KismetSystemLibrary.PrintText` (`|FormatText` "Targeting detected {Actor} with no ASC" _array_element) true true (struct :`R` 1.0 :`A` 1.0) 5.0)))))
            (:`Cancelled`
              (`KismetSystemLibrary.PrintString` "Wait Target Data Cancelled" true true (struct :`R` 1.0 :`A` 1.0) 5.0))))))
    (:`OnCompleted`
      (`self.K2_EndAbility` :!label _label))
    (:`OnBlendOut`
      (goto _label))
    (:`OnInterrupted`
      (goto _label))
    (:`OnCancelled`
      (goto _label))))

(event `self.K2_OnEndAbility`
  (params (bWasCancelled :type Boolean))
  (`KismetSystemLibrary.PrintText` (`|FormatText` "End TestAttack (Cancelled: {Cancelled})" bWasCancelled) true true (struct :`R` 1.0 :`A` 1.0) 5.0))