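; Gameplay ability that plays a slash montage and spawns a test projectile from the character's right-hand socket.
; ActivateAbility spawns BP_ProjectileTest with authority-only spawning as the montage starts, then ends the ability on montage completion.
; A disconnected path waits for a melee gameplay event to launch a hand-attached BP_Projectile carrying a damage effect spec along the view direction.
; Debug prints remain, including a server-side missed-event message on ability end.
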(event `Event LaunchSimple`
  (bind _ascharacter (cast `Character` (`self.GetAvatarActorFromActorInfo`)))
  (bind (_returnvalue_location _returnvalue_rotation) (`KismetMathLibrary.BreakTransform` (`SceneComponent.GetSocketTransform` (`Character.Mesh` _ascharacter) "RightHandSocket" "RTS_World")))
  ;[1 1 1] Defaults actor scale on server to 1,1,1
  (`GameplayTask_SpawnActor.SpawnActor` null _returnvalue_location _returnvalue_rotation "/Game/Marooned/Blueprints/Projectile/BP_ProjectileTest.BP_ProjectileTest_C" true _ascharacter))

(event `self.K2_ActivateAbility`
  (bind _asynctaskproxy (`AbilityTask_PlayMontageAndWait.CreatePlayMontageAndWaitProxy` "None" "/Game/Marooned/Characters/Man/AM_Man_Slash.AM_Man_Slash")
    (:`then`
      (`self.Event LaunchSimple`))
    (:`OnCompleted`
      (`self.NewMacro` false :!label _label
        (:`EndAbility`
          (`self.K2_EndAbility`))))
    (:`OnBlendOut`
      (goto _label :!via `BlendOut`))
    (:`OnInterrupted`
      (goto _label :!via `Interrupted`))
    (:`OnCancelled`
      (goto _label :!via `Cancelled`))))

(event `self.K2_OnEndAbility`
  (params (bWasCancelled :type Boolean))
  (if (`self.bDone`)
    _
    (elif (`Actor.HasAuthority` (`self.GetOwningActorFromActorInfo`))
      (`KismetSystemLibrary.PrintText` "Event Not Recieved"))))

(event `Event SpawnProjectile`
  (bind _ascharacter (cast `Character` (`self.GetAvatarActorFromActorInfo`)))
  (bind _mesh (`Character.Mesh` _ascharacter))
  (bind (_returnvalue_location _returnvalue_rotation) (`KismetMathLibrary.BreakTransform` (`SceneComponent.GetSocketTransform` _mesh "RightHandSocket" "RTS_World")))
  (bind (_asynctaskproxy _spawnedactor) (`GameplayTask_SpawnActor.SpawnActor` null _returnvalue_location _returnvalue_rotation "/Game/Marooned/Blueprints/Projectile/BP_Projectile.BP_Projectile_C" true _ascharacter)
    (:`Success`
      (bind _asbp_projectile (cast `/Game/Marooned/Blueprints/Projectile/BP_Projectile` _spawnedactor)
        (:`then`
          (bind _output_get (set `self.SpawnedProjectile` _asbp_projectile))
          (`Actor.K2_AttachToComponent` _output_get _mesh "RightHandSocket" "KeepWorld" "KeepWorld" "KeepWorld" true)
          (set `/Game/Marooned/Blueprints/Projectile/BP_Projectile.EffectSpecHandle` (`self.MakeOutgoingGameplayEffectSpec` "/Game/Marooned/Blueprints/GameplayAbilitySystem/Effects/BP_GE_Damage.BP_GE_Damage_C") _asbp_projectile))
        (:`CastFailed`
          (`KismetSystemLibrary.PrintString` "Cast Failed"))))))

(event `Event LaunchProjectile`
  (bind _spawnedprojectile (`self.SpawnedProjectile`)
    (:`then`
      (`Actor.K2_DetachFromActor` _spawnedprojectile "KeepWorld" "KeepWorld" "KeepWorld")
      (`/Game/Marooned/Blueprints/Projectile/BP_Projectile.Event Launch` _spawnedprojectile (`KismetMathLibrary.GetForwardVector` (`.OutRotation` (`Actor.GetActorEyesViewPoint` (`self.GetAvatarActorFromActorInfo`))))))
    (:`else`)))