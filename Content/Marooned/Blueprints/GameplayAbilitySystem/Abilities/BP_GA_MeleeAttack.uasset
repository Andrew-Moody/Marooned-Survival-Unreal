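; Melee attack gameplay ability that plays a slash montage and ends when it finishes or is interrupted.
; An Event.Attack.Melee gameplay event during the montage triggers an instant, short single-line trace from the avatar, filtering out self.
; Each target with an ability system applies damage and stun to itself, with hit-result context, then receives a knockback event.
; Debug prints remain, and a server-side bridge to the old resource attack is disconnected.
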(event `self.K2_ActivateAbility`
  (bind _returnvalue (`self.GetAvatarActorFromActorInfo`))
  ;[1 1 1] Play an animation and wait for anim event to trigger hit detection
  (`AbilityTask_PlayMontageAndWait.CreatePlayMontageAndWaitProxy` "None" "/Game/Marooned/Characters/Man/AM_Man_Slash.AM_Man_Slash"
    (:`then`
      (`AbilityTask_WaitGameplayEvent.WaitGameplayEvent` (struct :`TagName` "Event.Attack.Melee") null true false
        (:`EventReceived`
          (`|ExecutionSequence`
            (:`then_1`
              ;[1 1 1] Find Targets
              (bind (_asynctaskproxy _data) (`AbilityTask_WaitTargetData.WaitTargetData` "None" "Instant" "/Script/GameplayAbilities.GameplayAbilityTargetActor_SingleLineTrace" 300.0 (struct :`Name` "TargetPawn") true (make `GameplayAbilityTargetingLocationInfo` "ActorTransform" "0.000000,0.000000,0.000000|0.000000,0.000000,-0.000000|1.000000,1.000000,1.000000" _returnvalue) (struct) null (`AbilitySystemBlueprintLibrary.MakeFilterHandle` (make `GameplayTargetDataFilter` null "TDFS_NoSelf") _returnvalue))
                (:`ValidData`
                  (bind _returnvalue_2 (`AbilitySystemBlueprintLibrary.GetDataCountFromTargetData` _data))
                  ;[1 1 1] Apply Effects to all targets
                  (`KismetSystemLibrary.PrintText` (`|FormatText` "Data Count: {Count}" _returnvalue_2))
                  (for _index (range _returnvalue_2)
                    (`self.ApplyEffects` _data _index)))))))))
    (:`OnCompleted`
      (`self.K2_EndAbility` :!label _label))
    (:`OnBlendOut`
      (goto _label))
    (:`OnInterrupted`
      (goto _label))
    (:`OnCancelled`
      (goto _label))))

(fn `ApplyEffects`
  (params (TargetData :type "GameplayAbilityTargetDataHandle Structure") (Index :type Integer))
  (locals (HitResult :type "HitResult Structure") (TargetActor :type "Actor Object Reference") (TargetASC :type "AbilitySystemComponent Object Reference") (EffectContext :type "GameplayEffectContextHandle Structure"))
  (bind _effectcontext (`local.EffectContext`))
  (bind _targetasc (`local.TargetASC`))
  (bind (_bblockinghit _binitialoverlap _time _distance _location _impactpoint _normal _impactnormal _physmat _hitactor _hitcomponent _hitbonename _bonename _hititem) (`GameplayStatics.BreakHitResult` (`local.HitResult`)))
  (`KismetSystemLibrary.PrintText` (`|FormatText` "Data Count: {Count}" (`AbilitySystemBlueprintLibrary.GetDataCountFromTargetData` TargetData)))
  (set `local.HitResult` (`AbilitySystemBlueprintLibrary.GetHitResultFromTargetData` (`local.TargetData`) (`local.Index`)))
  (`KismetSystemLibrary.PrintText` (`|FormatText` "Hit Actor: {Actor}, Component: {Component}, Index: {Index}" (`KismetSystemLibrary.GetObjectName` _hitactor) (`KismetSystemLibrary.GetObjectName` _hitcomponent) _hititem))
  (for _array_element (`AbilitySystemBlueprintLibrary.GetActorsFromTargetData` (`local.TargetData`) (`local.Index`))
    (bind _output_get (set `local.TargetActor` _array_element))
    (bind _output_get_2 (set `local.TargetASC` (`AbilitySystemBlueprintLibrary.GetAbilitySystemComponent` _output_get)))
    (`/Engine/EditorBlueprintResources/StandardMacros.IsValid` _output_get_2
      (:`Is Valid`
        (bind _output_get_3 (set `local.EffectContext` (`AbilitySystemComponent.MakeEffectContext` (`local.TargetASC`))))
        (`AbilitySystemBlueprintLibrary.EffectContextAddHitResult` _output_get_3 (`local.HitResult`))
        (`AbilitySystemComponent.BP_ApplyGameplayEffectToSelf` _targetasc "/Game/Marooned/Blueprints/GameplayAbilitySystem/Effects/BP_GE_Damage.BP_GE_Damage_C" 0.0 _effectcontext)
        (`AbilitySystemComponent.BP_ApplyGameplayEffectToSelf` _targetasc "/Game/Marooned/Blueprints/GameplayAbilitySystem/Effects/BP_GE_Stun.BP_GE_Stun_C" 0.0 _effectcontext)
        ;[1 1 1] Send an event to trigger knockback
        (`AbilitySystemBlueprintLibrary.SendGameplayEventToActor` (`ActorComponent.GetOwner` (`local.TargetASC`)) (struct :`TagName` "Event.Debuff.Knockback") (make `GameplayEventData` (struct :`TagName` "Event.Debuff.Knockback") (`self.GetAvatarActorFromActorInfo`) (`local.TargetActor`))))
      (:`Is Not Valid`
        (`KismetSystemLibrary.PrintString` "Failed to find Ability System Component for Target")))))