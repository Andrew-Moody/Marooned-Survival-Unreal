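; Gameplay ability that handles death for AI and player characters.
; When activated from an event, it applies the Dying effect to itself, waits briefly, removes effects tagged State.Dying and applies the Dead effect.
; It then triggers ragdoll on the avatar, trying the AI character class first and falling back to the player character.
; It prints a debug string on activation and never calls EndAbility.
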(event `self.K2_ActivateAbilityFromEvent`
  (params (EventData :type "GameplayEventData Structure (by ref)"))
  (bind _returnvalue (`self.GetAvatarActorFromActorInfo`))
  (set `self.ASC` (`self.GetAbilitySystemComponentFromActorInfo`))
  (`KismetSystemLibrary.PrintString` "Death Activated")
  (`AbilitySystemComponent.BP_ApplyGameplayEffectToSelf` (`self.ASC`) "/Game/Marooned/Blueprints/GameplayAbilitySystem/Effects/BP_GE_Dying.BP_GE_Dying_C" 0.0 (make `GameplayEffectContextHandle`))
  (`AbilityTask_WaitDelay.WaitDelay` 0.05
    (:`OnFinish`
      (`AbilitySystemComponent.RemoveActiveEffectsWithTags` (`self.ASC`) (struct :`GameplayTags` (struct :`(TagName` "State.Dying"))))
      (`AbilitySystemComponent.BP_ApplyGameplayEffectToSelf` (`self.ASC`) "/Game/Marooned/Blueprints/GameplayAbilitySystem/Effects/BP_GE_Dead.BP_GE_Dead_C" 0.0 (make `GameplayEffectContextHandle`))
      (bind _asbp_gas_aicharacter (cast `/Game/Marooned/Blueprints/GameplayAbilitySystem/BP_GAS_AICharacter` _returnvalue)
        (:`then`
          (`/Game/Marooned/Blueprints/GameplayAbilitySystem/BP_GAS_AICharacter.Event Ragdoll` _asbp_gas_aicharacter))
        (:`CastFailed`
          (bind _asbp_gas_player_character (cast `/Game/Marooned/Blueprints/GameplayAbilitySystem/BP_GAS_PlayerCharacter` _returnvalue))
          (`/Game/Marooned/Blueprints/GameplayAbilitySystem/BP_GAS_PlayerCharacter.Event Ragdoll` _asbp_gas_player_character))))))