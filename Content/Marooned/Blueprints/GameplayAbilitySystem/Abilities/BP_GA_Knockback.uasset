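; BP_GA_Knockback is an event-triggered Gameplay Ability that knocks a character back, away from the event's instigator.
; On activation it prints a debug message, then builds a direction from the normalized instigator-to-target vector plus an upward bias.
; An ApplyRootMotionConstantForce task uses that direction with the Strength and Duration variables, keeps the last root motion velocity on finish, and then ends the ability.
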(event `self.K2_ActivateAbilityFromEvent`
  (params (EventData :type "GameplayEventData Structure (by ref)"))
  (bind (_eventtag _instigator _target) (break `GameplayEventData` EventData))
  (`KismetSystemLibrary.PrintString` "Event Recieved" true true (struct :`G` 1.0 :`A` 1.0) 5.0)
  (`AbilityTask_ApplyRootMotionConstantForce.ApplyRootMotionConstantForce` "None" (+ (0.0 0.0 0.5) (`KismetMathLibrary.Normal` (- (`Actor.K2_GetActorLocation` _target) (`Actor.K2_GetActorLocation` _instigator)))) (`self.Strength`) (`self.Duration`) false null "MaintainLastRootMotionVelocity"
    (:`OnFinish`
      (`self.K2_EndAbility`))))