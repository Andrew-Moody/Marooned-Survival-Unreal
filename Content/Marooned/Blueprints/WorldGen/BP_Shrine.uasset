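; BP_Shrine is an interactable shrine that summons a goblin enemy and rewards a max health powerup when it is killed.
; On Interact, the authority spawns BP_Enemy_Goblin beside the shrine, only if no valid summoned enemy already exists.
; It binds to that enemy's death dispatcher, which spawns the powerup above the shrine and then destroys the shrine.
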(event `Event Interact`
  (`self.SpawnEnemy`
    (:`then`)
    (:`else`
      (`/Engine/EditorBlueprintResources/ActorMacros.Switch Has Authority`
        (:`Authority`
          (bind _returnvalue (`|SpawnActorFromClass` "/Game/Marooned/Characters/Goblin/BP_Enemy_Goblin.BP_Enemy_Goblin_C" (`KismetMathLibrary.MakeTransform` (+ (.location (`self.GetTransform`)) (200.0 0.0 100.0)) (.rotation (`self.GetTransform`)) (.scale (`self.GetTransform`))) "AlwaysSpawn" "OverrideRootScale" null null))
          (bind _output_get (set `self.SpawnEnemy` _returnvalue))
          (add `/Game/Marooned/Blueprints/GameplayAbilitySystem/BP_GAS_AICharacter.DeathEventDispatcher` _output_get (delegate `CustomEvent`)))))))

(event `CustomEvent`
  (`|SpawnActorFromClass` "/Game/Marooned/Blueprints/Powerups/BP_Powerup_MaxHealth.BP_Powerup_MaxHealth_C" (`KismetMathLibrary.MakeTransform` (+ (.location (`self.GetTransform`)) (0.0 0.0 150.0)) (.rotation (`self.GetTransform`)) (.scale (`self.GetTransform`))) "AlwaysSpawn" "OverrideRootScale" null null)
  (`self.K2_DestroyActor`))

(fn `UserConstructionScript`)