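; BP_TerrainManager scatters Blood and Spruce resources across a square grid in the world at BeginPlay.
; Grid points where the product of two 1D Perlin noise samples meets a threshold are line-traced vertically to find the ground.
; A seeded random stream sorts each hit into one of two transform arrays, which are then handed to their Clusters for batch population.
; The checkerboard PickResource and timing printout are disconnected.
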(event `self.ReceiveBeginPlay`
  (`KismetMathLibrary.SetRandomStreamSeed` (`self.RandomStream`) (`self.Seed`))
  (`self.Event Populate`))

(event `Event Populate`
  (bind _returnvalue (- (`self.SideCount`) 1))
  (bind (_x _y) (`KismetMathLibrary.BreakVector3f` (.location (`self.GetTransform`))))
  (set `self.Xoffset` _x)
  (set `self.Yoffset` _y)
  (`|ExecutionSequence`
    (:`then_0`
      (`self.CheckTime` false)
      (for _index (range (+ _returnvalue 1))
        (for _index_2 (range (+ _returnvalue 1))
          (`self.TryPlaceResource` _index _index_2 (+ (`KismetMathLibrary.Conv_IntToDouble` (* _index 300)) (`self.Yoffset`)) (+ (`KismetMathLibrary.Conv_IntToDouble` (* _index_2 300)) (`self.Xoffset`))))))
    (:`then_1`
      (`self.CheckTime` true)
      (`/Game/Marooned/Blueprints/WorldGen/BP_TreeISM.Populate` (`BlueprintMapLibrary.Map_Find` (`self.Clusters`)) (`self.BloodTransforms`))
      (`/Game/Marooned/Blueprints/WorldGen/BP_TreeISM.Populate` (`BlueprintMapLibrary.Map_Find` (`self.Clusters`) 1) (`self.SpruceTransforms`))
      (`self.CheckTime` true))))

(fn `CheckTime`
  (params (bPrintDiff :type Boolean))
  (bind (_seconds _partialseconds) (`GameplayStatics.GetAccurateRealTime`))
  (`|ExecutionSequence`
    (:`then_0`
      (if bPrintDiff
        _))
    (:`then_1`
      (set `self.PrevTime` (+ _seconds _partialseconds)))))

(fn `PickResource`
  (params (X :type Integer) (Y :type Integer))
  (returns (Id :type Integer))
  (if (xor (== (mod X 2) 0) (== (mod Y 2) 0))
    (return 0)
    (else
      (return 1))))

(fn `TryPlaceResource`
  (params (XIndex :type Integer) (YIndex :type Integer) (XCoord :type "Float (double-precision)") (YCoord :type "Float (double-precision)"))
  (bind _noisescale (`self.NoiseScale`))
  (if (>= (* (`KismetMathLibrary.PerlinNoise1D` (* (+ XIndex 37) _noisescale)) (`KismetMathLibrary.PerlinNoise1D` (* YIndex _noisescale))) (`self.Threshold`))
    (bind (_outhit _returnvalue) (`KismetSystemLibrary.LineTraceSingle` (`KismetMathLibrary.MakeVector` XCoord YCoord 500.0) (`KismetMathLibrary.MakeVector` XCoord YCoord -500.0) "TraceTypeQuery2"))
    (if _returnvalue
      (switch `int` (`KismetMathLibrary.RandomIntegerInRangeFromStream` 0 1 (`self.RandomStream`))
        (:`0`
          (bind _returnvalue_2 (`KismetMathLibrary.MakeTransform` (`.Location` (`GameplayStatics.BreakHitResult` _outhit))))
          (`KismetArrayLibrary.Array_Add` (`self.BloodTransforms`) _returnvalue_2))
        (:`1`
          (`KismetArrayLibrary.Array_Add` (`self.SpruceTransforms`) _returnvalue_2))))))

(fn `UserConstructionScript`)