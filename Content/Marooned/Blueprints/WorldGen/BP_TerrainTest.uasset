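; BP_TerrainTest is a terrain test driver that triggers populate on a list of Managers one at a time and times the run.
; Tick calls SpawnNextChunk when not Loading, which sets the flag and advances through the array.
; Nothing connected here clears Loading after a populate starts.
; CheckTime records real time at BeginPlay and prints elapsed seconds once the list is exhausted and Loading is false.
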(event `Key|M`
  (params (Key :type "Key Structure")))

(event `self.ReceiveBeginPlay`
  (`self.EnableInput` (`GameplayStatics.GetPlayerController` 0))
  (`self.CheckTime` false)
  (set `self.bLoading` false))

(event `self.ReceiveTick`
  (params (DeltaSeconds :type "Float (single-precision)"))
  (bind _returnvalue (not (`self.bLoading`)))
  (bind _returnvalue_2 (< (`self.Index`) (`KismetArrayLibrary.Array_Length` (`self.Managers`))))
  (if (and _returnvalue _returnvalue_2)
    (`self.Event SpawnNextChunk`)
    (elif (and _returnvalue (not _returnvalue_2))
      (`/Engine/EditorBlueprintResources/StandardMacros.DoOnce` false
        (:`Completed`
          (`self.CheckTime` true))))))

(event `Event SpawnNextChunk`
  (set `self.bLoading` true)
  (if (< (`self.Index`) (`KismetArrayLibrary.Array_Length` (`self.Managers`)))
    (`/Game/Marooned/Blueprints/WorldGen/BP_TerrainManager.Event Populate` (`|GetArrayItem` (`self.Managers`) (`self.Index`)))
    (`/Engine/EditorBlueprintResources/StandardMacros.IncrementInt` (`self.Index`))))

(fn `CheckTime`
  (params (bPrintDiff :type Boolean))
  (bind (_seconds _partialseconds) (`GameplayStatics.GetAccurateRealTime`))
  (bind _returnvalue (+ _seconds _partialseconds))
  (`|ExecutionSequence`
    (:`then_0`
      (if bPrintDiff
        (`KismetSystemLibrary.PrintText` (`|FormatText` "Time Elapsed: {Seconds} Seconds" (- _returnvalue (`self.PrevTime`))) true true (struct :`G` 0.66 :`B` 1.0 :`A` 1.0) 15.0)))
    (:`then_1`
      (set `self.PrevTime` _returnvalue))))

(fn `UserConstructionScript`)