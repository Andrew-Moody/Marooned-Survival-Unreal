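; Procedural terrain mesh actor that builds a welded grid and displaces its height with noise.
; UpdateMesh stores the parameters, calls Resize to rebuild the collision-enabled section when the vertex count changes, sets heights, then updates the section.
; Height multiplies two 1D Perlin samples, one per axis; Seed is stored but unused.
; Normal and tangent recalculation is disconnected, as is CheckTime's timing printout, and construction only prints a message.
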(event `UpdateMesh`
  (params (Seed :type Integer) (Size :type Integer) (NoiseScale :type "Float (double-precision)") (Height :type "Float (double-precision)"))
  (bind _noisescale (`self.NoiseScale`))
  (bind _size (`self.Size`))
  (bind _returnvalue (+ (`self.Size`) 1))
  (set `self.Seed` Seed)
  (set `self.Size` Size)
  (set `self.NoiseScale` NoiseScale)
  (set `self.Height` Height)
  (`|ExecutionSequence`
    (:`then_0`
      (if (!= (* _returnvalue _returnvalue) (`KismetArrayLibrary.Array_Length` (`self.Vertices`)))
        (`self.Resize`)))
    (:`then_1`
      (`self.CheckTime` false)
      ;[1 1 1] Modify Heights with Noise
      (for _index (range (+ (`self.Size`) 1))
        (for _index_2 (range (+ _size 1))
          (bind _output (`|GetArrayItem` (`self.Vertices`) (+ _index_2 (* _index _size))))
          (`KismetMathLibrary.Vector_Set` _output (.x _output) (.y _output) (* (`KismetMathLibrary.PerlinNoise1D` (* _noisescale _index)) (`KismetMathLibrary.PerlinNoise1D` (* _noisescale _index_2)) (`self.Height`)))))
      (`self.CheckTime` false "Setting Heights"))
    (:`then_2`
      (`self.CheckTime` false)
      (`ProceduralMeshComponent.UpdateMeshSection_LinearColor` :`self` (`self.ProceduralMesh`) :`Vertices` (`self.Vertices`) :`Normals` (`self.Normals`) :`UV0` (`self.UV0`) :`Tangents` (`self.Tangents`) :`bSRGBConversion` false)
      (`self.CheckTime` false "Updating Mesh"))))

(fn `CheckTime`
  (params (bPrintDiff :type Boolean) (Prefix :type String))
  (bind (_seconds _partialseconds) (`GameplayStatics.GetAccurateRealTime`))
  (`|ExecutionSequence`
    (:`then_0`
      (if bPrintDiff
        _))
    (:`then_1`
      (set `self.PrevTime` (+ _seconds _partialseconds)))))

(fn `Resize`
  (bind _returnvalue (+ (`self.Size`) 1))
  (`|ExecutionSequence`
    (:`then_1`
      (`self.CheckTime` false)
      ;[1 1 1] Create Triangles, Normals, and Tangents then Create a Mesh Section
      (bind (_triangles _vertices _uvs) (`KismetProceduralMeshLibrary.CreateGridMeshWelded` _returnvalue _returnvalue 100.0))
      (set `self.Triangles` _triangles)
      (set `self.Vertices` _vertices)
      (set `self.UV0` _uvs)
      (`self.CheckTime` false "Create Grid")
      (`ProceduralMeshComponent.CreateMeshSection_LinearColor` :`self` (`self.ProceduralMesh`) :`Vertices` (`self.Vertices`) :`Triangles` (`self.Triangles`) :`UV0` (`self.UV0`) :`bCreateCollision` true)
      (`PrimitiveComponent.SetMaterial` (`self.ProceduralMesh`) 0 "/Game/Marooned/Characters/M_LowPolyPalette.M_LowPolyPalette")
      (`self.CheckTime` false "Create Mesh Section"))
    (:`then_2`
      (return))))

(fn `UserConstructionScript`
  (locals (NewLocalVar :type Integer))
  (`KismetSystemLibrary.PrintString` "Mesh Construction Called"))