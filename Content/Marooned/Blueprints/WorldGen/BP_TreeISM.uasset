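; Instanced-mesh manager for harvestable trees that fills a grid on BeginPlay and tracks health and alive state per instance.
; Attacks lower the hit instance's health, dim its custom data value to hide it, and spawn a temporary spruce actor to play hit effects.
; When effects finish, the instance reappears and the actor is destroyed; at zero health, the authority spawns a world item and culls the instance by moving its transform.
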(event `self.ReceiveBeginPlay`
  (set `self.ISMRef` (`self.InstancedStaticMesh`))
  (`StaticMeshComponent.SetStaticMesh` (`self.ISMRef`) (`self.StaticMesh`))
  (for _index (range 101)
    (for _index_2 (range 101)
      (`KismetArrayLibrary.Array_Add` (`self.Instances`) (make `/Game/Marooned/Blueprints/WorldGen/F_ResourceInstance` true 3.0))
      (bind _returnvalue (`InstancedStaticMeshComponent.AddInstance` (`self.ISMRef`) (`KismetMathLibrary.MakeTransform` (`KismetMathLibrary.MakeVector` (`KismetMathLibrary.Conv_IntToDouble` (* _index_2 200)) (`KismetMathLibrary.Conv_IntToDouble` (* _index 200)))) true))
      (`InstancedStaticMeshComponent.SetCustomDataValue` (`self.ISMRef`) _returnvalue 0 1.0 false))))

(event `/Game/Marooned/Blueprints/WorldGen/BPI_Attack.Attack`
  (params (HitResult :type "HitResult Structure") (Damage :type "Float (double-precision)"))
  (bind _output_get (set `self.HitResult` HitResult))
  (set `self.Damage` Damage)
  (set `self.InstanceIndex` (`.HitItem` (`GameplayStatics.BreakHitResult` _output_get)))
  (`self.Event AttackInstance` (`self.InstanceIndex`) (`self.HitResult`) (`self.Damage`) (`KismetMathLibrary.FClamp` (- (`self.GetHealth` (`self.InstanceIndex`)) (`self.Damage`)) 0.0 100.0)))

(event `Event ActorExpire`
  (params (InstanceIndex :type Integer))
  ;[1 1 1] Show the instance corresponding to the expired actor
  (`self.Event ShowInstance` InstanceIndex))

(event `Event ActorDeath`
  (params (InstanceIndex :type Integer))
  ;[1 1 1] Cull the instance corresponding to the dead actor
  (`self.Event CullInstance` InstanceIndex))

(event `Event HideInstance`
  (params (InstanceIndex :type Integer))
  ;[1 1 1] Multicast RPCs for showing, hiding, and culling instances
  (`self.HideInstance` InstanceIndex))

(event `Event AttackInstance`
  (params (InstanceIndex :type Integer) (HitResult :type "HitResult Structure") (Damage :type "Float (double-precision)") (NewHealth :type "Float (double-precision)"))
  (`|ExecutionSequence`
    (:`then_0`
      (`self.SetHealth` InstanceIndex NewHealth)
      (`self.HealthChanged` InstanceIndex NewHealth)
      (`self.HideInstance` InstanceIndex))
    (:`then_1`
      (bind _returnvalue (`|SpawnActorFromClass` "/Game/Marooned/Blueprints/WorldGen/Resources/BP_Resource_Spruce.BP_Resource_Spruce_C" (`InstancedStaticMeshComponent.GetInstanceTransform` (`self.ISMRef`) InstanceIndex true) "Undefined" "OverrideRootScale" null self InstanceIndex null))
      (`/Game/Marooned/Blueprints/WorldGen/BP_Resource.Event PlayAttackFX` _returnvalue HitResult Damage))))

(event `Event ShowInstance`
  (params (InstanceIndex :type Integer))
  ;[1 1 1] Multicast RPCs for showing, hiding, and culling instances
  (`self.ShowInstance` InstanceIndex))

(event `Event CullInstance`
  (params (InstanceIndex :type Integer))
  ;[1 1 1] Multicast RPCs for showing, hiding, and culling instances
  (`self.CullInstance` InstanceIndex))

(event `Event FinishedAttackFX`
  (params (InstanceIndex :type Integer) (BP_Resource :type "/Game/Marooned/Blueprints/WorldGen/BP_Resource Object Reference"))
  (`self.ShowInstance` InstanceIndex)
  (`self.K2_DestroyActor` BP_Resource)
  (`/Engine/EditorBlueprintResources/ActorMacros.Switch Has Authority`
    (:`Authority`
      (if (<= (`self.GetHealth` InstanceIndex) 0.0)
        (`|SpawnActorFromClass` "/Game/Marooned/Blueprints/Item/BP_WorldItem.BP_WorldItem_C" (`KismetMathLibrary.ComposeTransforms` (`InstancedStaticMeshComponent.GetInstanceTransform` (`self.ISMRef`) InstanceIndex true) (`KismetMathLibrary.MakeTransform` (0.0 0.0 100.0))) "AlwaysSpawn" "OverrideRootScale" null null)
        (`self.Event ActorDeath` InstanceIndex)))))

(fn `CullInstance`
  (params (InstanceIndex :type Integer))
  (setmembers `/Game/Marooned/Blueprints/WorldGen/F_ResourceInstance` :`StructRef` (`|GetArrayItem` (`self.Instances`) InstanceIndex) :`bAlive` false)
  (`InstancedStaticMeshComponent.UpdateInstanceTransform` (`self.ISMRef`) InstanceIndex (`self.CullTransform`) true true true))

(fn `GetHealth`
  (params (`Instance Index` :type Integer))
  (returns (Health :type "Float (double-precision)"))
  (if (> `Instance Index` -1)
    (return (`.Health_7_08975BAE42C51639FB235EB3E5A7F5CB` (break `/Game/Marooned/Blueprints/WorldGen/F_ResourceInstance` (`|GetArrayItem` (`self.Instances`) `Instance Index`))))
    (else
      (return -1.0))))

(fn `HideInstance`
  (params (InstanceIndex :type Integer))
  (`KismetSystemLibrary.PrintText` (`|FormatText` "Hide Instance {Index}" InstanceIndex))
  (bind _returnvalue (`InstancedStaticMeshComponent.SetCustomDataValue` (`self.ISMRef`) InstanceIndex 0 0.2 true))
  (`KismetSystemLibrary.PrintString` (`KismetStringLibrary.Conv_BoolToString` _returnvalue)))

(fn `SetHealth`
  (params (`Instance Index` :type Integer) (Health :type "Float (double-precision)"))
  (setmembers `/Game/Marooned/Blueprints/WorldGen/F_ResourceInstance` :`StructRef` (`|GetArrayItem` (`self.Instances`) `Instance Index`) :`Health` Health))

(fn `ShowInstance`
  (params (InstanceIndex :type Integer))
  (`KismetSystemLibrary.PrintText` (`|FormatText` "Show Instance {Index}" InstanceIndex))
  (`InstancedStaticMeshComponent.SetCustomDataValue` (`self.ISMRef`) InstanceIndex 0 1.0 true))

(fn `UserConstructionScript`)