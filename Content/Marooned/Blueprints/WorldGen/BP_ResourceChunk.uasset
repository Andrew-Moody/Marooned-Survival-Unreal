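; World-gen chunk actor that handles health and destruction events for instanced resources held in MUResourceInstanceComponents.
; When a resource is destroyed, it spawns a BP_WorldItem at that transform, always with the Bloodwood Log data asset, and prints a debug message.
; Health requests and change notifications both read per-instance health and the data asset's starting health, then call HealthChanged with an actor proxy handle identifying the instance.
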(event `self.ReceiveBeginPlay`)

(event `self.RecieveResourceDestroyed`
  (params (Transform :type "Transform Structure"))
  (`|SpawnActorFromClass` "/Game/Marooned/Blueprints/Item/BP_WorldItem.BP_WorldItem_C" Transform "Undefined" "OverrideRootScale" null "/Game/Marooned/DataAssets/Items/DA_Item_BloodwoodLog.DA_Item_BloodwoodLog" null)
  (`KismetSystemLibrary.PrintString` "SpawningItem" true true (struct :`G` 0.66 :`B` 1.0 :`A` 1.0) 10.0))

(event `Event RequestHealthUpdate`
  (params (ActorProxyHandle :type "ActorProxyHandle Structure"))
  (bind (_actor _component _index) (break `ActorProxyHandle` ActorProxyHandle))
  (bind _asmuresource_instance_component (cast `MUResourceInstanceComponent` _component))
  (bind _returnvalue (`MUResourceInstanceComponent.GetHealth` _asmuresource_instance_component _index))
  (`self.HealthChanged` _returnvalue (`ResourceDataAsset.StartingHealth` (`MUResourceInstanceComponent.DataAsset` _asmuresource_instance_component)) ActorProxyHandle))

(event `self.RecieveResourceHealthChanged`
  (params (Component :type "MUResourceInstanceComponent Object Reference") (InstanceIndex :type Integer))
  (bind _returnvalue (`MUResourceInstanceComponent.GetHealth` Component InstanceIndex))
  (`self.HealthChanged` _returnvalue (`ResourceDataAsset.StartingHealth` (`MUResourceInstanceComponent.DataAsset` Component)) (make `ActorProxyHandle` self Component InstanceIndex)))

(fn `UserConstructionScript`)