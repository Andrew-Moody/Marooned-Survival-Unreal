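; BP_ResourcePerfTest is a world-generation performance test actor for resources represented as instanced static meshes.
; BeginPlay fills the ISM with a square, evenly spaced grid of Bloodwood tree instances, sized by the Size variable.
; ActivateInstance spawns a BP_Resource_Spruce actor at an instance's world transform, leaving the instance in place.
; DeactivateInstance is an empty stub.
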(event `self.ReceiveBeginPlay`
  (`StaticMeshComponent.SetStaticMesh` (`self.ISM`) "/Game/Marooned/Terrain/Trees_Tree_Bloodwood.Trees_Tree_Bloodwood")
  (for _index (range (+ (`self.Size`) 1))
    (for _index_2 (range (+ (`self.Size`) 1))
      (`InstancedStaticMeshComponent.AddInstance` (`self.ISM`) (`KismetMathLibrary.MakeTransform` (`KismetMathLibrary.MakeVector` (* _index 200.0) (* _index_2 200.0))) true))))

(event `ActivateInstance`
  (params (`Instance Index` :type Integer))
  (`|SpawnActorFromClass` "/Game/Marooned/Blueprints/WorldGen/Resources/BP_Resource_Spruce.BP_Resource_Spruce_C" (`InstancedStaticMeshComponent.GetInstanceTransform` (`self.ISM`) `Instance Index` true) "Undefined" "OverrideRootScale" null null))

(event `DeactivateInstance`
  (params (`Instance Index` :type Integer)))

(fn `UserConstructionScript`)