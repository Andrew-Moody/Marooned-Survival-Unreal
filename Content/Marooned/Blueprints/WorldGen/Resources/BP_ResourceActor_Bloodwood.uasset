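; Bloodwood resource actor that supplies the visual feedback for being hit and for dying.
; Its hit and death events each spawn the same HitFX particle system at the impact point and play their own timeline to animate actor scale.
; Each timeline calls FinishFX on completion, which is required to finalize the effect.
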(event `self.StartHitFX_BPImpl`
  (params (HitResult :type "HitResult Structure (by ref)"))
  (`|ExecutionSequence`
    (:`then_0`
      (`NiagaraFunctionLibrary.SpawnSystemAtLocation` (`self.HitFX`) (`.ImpactPoint` (`GameplayStatics.BreakHitResult` HitResult))))
    (:`then_1`
      (bind (_direction _scale) (`Timeline|Timeline` :!via `PlayFromStart`)
        (:`Update`
          (`self.SetActorScale3D` _scale))
        (:`Finished`
          ;[1 1 1] Must Call FinishFX to finalize
          (`self.FinishFX`))))))

(event `self.StartDeathFX_BPImpl`
  (params (HitResult :type "HitResult Structure (by ref)"))
  (`|ExecutionSequence`
    (:`then_0`
      (`NiagaraFunctionLibrary.SpawnSystemAtLocation` (`self.HitFX`) (`.ImpactPoint` (`GameplayStatics.BreakHitResult` HitResult))))
    (:`then_1`
      (bind (_direction _scale) (`Timeline|Timeline_0` :!via `PlayFromStart`)
        (:`Update`
          (`self.SetActorScale3D` _scale))
        (:`Finished`
          ;[1 1 1] Must Call FinishFX to finalize
          (`self.FinishFX`))))))

(fn `UserConstructionScript`)