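; Terrain generator for Marooned's world generation that builds a noise-based terrain mesh from size, noise scale and height settings.
; The construction script calls Refresh, which uses UseNative to pick between BPTMesh, timed as "Native Update", and BPTerrainMesh.
; Only the BPTerrainMesh path receives Seed, and only BPTMesh receives TileSize.
; A separate BakeCollision event bakes collision on BPTMesh alone.
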(event `Bake Collision`
  (`/Game/Marooned/Blueprints/WorldGen/BP_TMesh.Bake Collison` (`self.BP_TMesh`)))

(event `Refresh`
  (bind _size (`self.Size`))
  (if (`self.bUseNative`)
    (`/Game/Marooned/Blueprints/WorldGen/BP_TerrainMesh.CheckTime` (`self.BP_TerrainMesh`) false "")
    (`TerrainMesh.UpdateMesh` (`self.BP_TMesh`) _size _size (`self.TileSize`) (`self.NoiseScale`) (`self.Height`))
    (`/Game/Marooned/Blueprints/WorldGen/BP_TerrainMesh.CheckTime` (`self.BP_TerrainMesh`) true "Native Update")
    (else
      (`/Game/Marooned/Blueprints/WorldGen/BP_TerrainMesh.UpdateMesh` (`self.BP_TerrainMesh`) (`self.Seed`) (`self.Size`) (`self.NoiseScale`) (`self.Height`)))))

(fn `UserConstructionScript`
  (`self.Refresh`))