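; AI controller for GAS-based enemy characters that runs the BT_Man behavior tree and feeds its blackboard.
; On possess it stores the pawn's ability system and listens for tag changes, setting bImmobalized from the State.Dead tag.
; Sight perception sets or clears the player as TargetActor and records LastSeenLocation when sight is lost.
; An AttackMontage RepNotify plays the montage on the controlled character.
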(event `self.AIPerception.OnTargetPerceptionUpdated`
  (params (Actor :type "Actor Object Reference") (Stimulus :type "AIStimulus Structure"))
  (`self.HandleSightSense` Actor Stimulus))

(event `self.ReceiveBeginPlay`
  (`self.RunBehaviorTree` "/Game/Marooned/Blueprints/AI/BT_Man.BT_Man"))

(event `self.ReceivePossess`
  (params (PossessedPawn :type "Pawn Object Reference"))
  (bind _returnvalue (`AbilitySystemBlueprintLibrary.GetAbilitySystemComponent` PossessedPawn))
  (bind _asbp_gas_aicharacter (cast `/Game/Marooned/Blueprints/GameplayAbilitySystem/BP_GAS_AICharacter` PossessedPawn))
  (add `/Game/Marooned/Blueprints/GameplayAbilitySystem/BP_GAS_AICharacter.TagChanged` _asbp_gas_aicharacter (delegate `EventTagChanged`))
  (`/Engine/EditorBlueprintResources/StandardMacros.IsValid` _returnvalue
    (:`Is Valid`
      (bind _output_get (set `self.ASC` _returnvalue))
      (`BlackboardComponent.SetValueAsObject` (`self.Blackboard`) "AbilitySystem" _output_get))))

(event `EventTagChanged`
  (params (ChangedTag :type "GameplayTag Structure") (NewCount :type Integer))
  (if (`BlueprintGameplayTagLibrary.MatchesAnyTags` ChangedTag (`BlueprintGameplayTagLibrary.MakeLiteralGameplayTagContainer` (struct :`GameplayTags` (struct :`(TagName` "State.Dead") :`(TagName` "State.Dying") :`(TagName` "Debuff.Stun")))) true)
    (`BlackboardComponent.SetValueAsBool` (`self.Blackboard`) "bImmobalized" (`GameplayTagAssetInterface.HasAnyMatchingGameplayTags` (`self.ASC`) (`BlueprintGameplayTagLibrary.MakeLiteralGameplayTagContainer` (struct :`GameplayTags` (struct :`(TagName` "State.Dead") :`(TagName` "State.Dying") :`(TagName` "Debuff.Stun"))))))))

(fn `HandleSightSense`
  (params (Actor :type "Actor Object Reference") (Stimulus :type "AIStimulus Structure"))
  (bind (_stimulus_age _stimulus_expirationage _stimulus_strength _stimulus_stimuluslocation _stimulus_receiverlocation _stimulus_tag _stimulus_bsuccessfullysensed) (break `AIStimulus` (`local.Stimulus`)))
  (bind _returnvalue (`AIPerceptionSystem.GetSenseClassForStimulus` Stimulus))
  (if (and (== _returnvalue "/Script/AIModule.AISense_Sight") (== Actor (`GameplayStatics.GetPlayerCharacter` 0)))
    (`BlackboardComponent.SetValueAsObject` (`self.Blackboard`) "TargetActor" (`KismetMathLibrary.SelectObject` (`GameplayStatics.GetPlayerCharacter` 0) null _stimulus_bsuccessfullysensed))
    (if (not _stimulus_bsuccessfullysensed)
      (`BlackboardComponent.SetValueAsVector` (`self.Blackboard`) "LastSeenLocation" _stimulus_stimuluslocation))
    (else
      (return))))

(fn `OnRep_AttackMontage`
  (bind (_montage _starttime _playrate _startsection) (break `/Game/Marooned/Blueprints/Core/F_MontageData` (`self.AttackMontage`)))
  (bind _ascharacter (cast `Character` (`self.K2_GetPawn`)))
  (`Character.PlayAnimMontage` _ascharacter _montage _playrate _startsection))

(fn `UserConstructionScript`)