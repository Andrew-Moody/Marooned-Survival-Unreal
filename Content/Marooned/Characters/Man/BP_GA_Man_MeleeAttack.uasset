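; Gameplay ability for the Man character's melee slash in Marooned.
; It plays the slash montage and, on each melee attack gameplay event, runs an instant radius targeting query around the avatar, excluding itself.
; Each target with an ability system component applies the goblin melee and stun effects to itself.
; The ability ends when the montage finishes or is interrupted; a knockback event send is present but unwired.
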(event `self.K2_ActivateAbility`
  (bind _returnvalue (`self.GetAvatarActorFromActorInfo`))
  (bind _gameplayeffectcontexthandle (make `GameplayEffectContextHandle`))
  ;[1 1 1] Play an animation and wait for anim event to trigger hit detection
  (`AbilityTask_PlayMontageAndWait.CreatePlayMontageAndWaitProxy` "None" "/Game/Marooned/Characters/Man/AM_Man_Slash.AM_Man_Slash"
    (:`then`
      (`AbilityTask_WaitGameplayEvent.WaitGameplayEvent` (struct :`TagName` "Event.Attack.Melee") null true false :!label _label
        (:`EventReceived`
          (`|ExecutionSequence`
            (:`then_0`
              ;[1 1 1] Find Targets
              (bind (_asynctaskproxy _data) (`AbilityTask_WaitTargetData.WaitTargetData` "None" "Instant" "/Script/GameplayAbilities.GameplayAbilityTargetActor_Radius" 150.0 (make `GameplayAbilityTargetingLocationInfo` "ActorTransform" "0.000000,0.000000,0.000000|0.000000,0.000000,-0.000000|1.000000,1.000000,1.000000" _returnvalue) (struct) null (`AbilitySystemBlueprintLibrary.MakeFilterHandle` (make `GameplayTargetDataFilter` null "TDFS_NoSelf") _returnvalue))
                (:`ValidData`
                  ;[1 1 1] Apply Effects to all targets
                  (for _array_element (`AbilitySystemBlueprintLibrary.GetAllActorsFromTargetData` _data)
                    (bind _returnvalue_2 (`AbilitySystemBlueprintLibrary.GetAbilitySystemComponent` _array_element))
                    (`/Engine/EditorBlueprintResources/StandardMacros.IsValid` _returnvalue_2
                      (:`Is Valid`
                        (`AbilitySystemComponent.BP_ApplyGameplayEffectToSelf` _returnvalue_2 "/Game/Marooned/Blueprints/GameplayAbilitySystem/Effects/BP_GE_Goblin_Melee.BP_GE_Goblin_Melee_C" 0.0 _gameplayeffectcontexthandle)
                        (`AbilitySystemComponent.BP_ApplyGameplayEffectToSelf` _returnvalue_2 "/Game/Marooned/Blueprints/GameplayAbilitySystem/Effects/BP_GE_Stun.BP_GE_Stun_C" 0.0 _gameplayeffectcontexthandle)))))))
            (:`then_1`
              (goto _label))))))
    (:`OnCompleted`
      (`self.K2_EndAbility` :!label _label_2))
    (:`OnBlendOut`
      (goto _label_2))
    (:`OnInterrupted`
      (goto _label_2))
    (:`OnCancelled`
      (goto _label_2))))